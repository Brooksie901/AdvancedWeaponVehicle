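; BP_Laser is a laser beam actor that extends forward until something blocks it.
; Each Tick it line-traces on Visibility along its forward vector, feeding the end point to the beam particle and showing the impact effect only on hits.
; Trace distance grows over time up to a cap and shortens to the hit distance when blocked, so the beam re-extends gradually.
; BeginPlay tints both effects orange; the trace's debug drawing is enabled.
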(event EventTick
  (params (DeltaSeconds :type Float%20%28single-precision%29))
  (bind _returnvalue (Transformation|GetActorLocation))
  (Utilities|FlowControl|Sequence
    (:then_0
      (Variables|Default|SetTraceEnd (+ _returnvalue (* (Transformation|GetActorForwardVector) (Variables|Default|GetTraceDisatnce))))
      (bind _outhit (Collision|LineTraceByChannel _returnvalue (+ _returnvalue (* (Transformation|GetActorForwardVector) (Variables|Default|GetTraceDisatnce))) "TraceTypeQuery1" false 0 "ForOneFrame"))
      (Variables|Default|SetHit (.bblockinghit _outhit))
      (Variables|Default|SetHitLocation (.location _outhit))
      (Effects|Components|ParticleSystem|SetVectorParameter (Variables|Default|GetLaser) "LaserEnd" (select (Variables|Default|GetHit) (Variables|Default|GetHitLocation) (Variables|Default|GetTraceEnd)))
      (Rendering|SetVisibility (Variables|Default|GetLaserImpact) (Variables|Default|GetHit) false)
      (Transformation|SetWorldLocation (Variables|Default|GetLaserImpact) (Variables|Default|GetHitLocation) false false)
      (if (Variables|Default|GetHit)
        (Variables|Default|SetTraceDisatnce (Math|Vector|VectorLength (- (Variables|Default|GetHitLocation) (Transformation|GetActorLocation))))))
    (:then_1
      (if (< (Variables|Default|GetTraceDisatnce) 5e+03)
        (Variables|Default|SetTraceDisatnce (+ (Variables|Default|GetTraceDisatnce) (* DeltaSeconds 2e+03)))))))

(event EventBeginPlay
  (Effects|Components|ParticleSystem|SetColorParameter (Variables|Default|GetLaser) "Colour" "(R=0.770833,G=0.238211,B=0.043996,A=1.000000)")
  (Effects|Components|ParticleSystem|SetColorParameter (Variables|Default|GetLaserImpact) "Colour" "(R=0.770833,G=0.226171,B=0.000000,A=1.000000)"))

(fn ConstructionScript)