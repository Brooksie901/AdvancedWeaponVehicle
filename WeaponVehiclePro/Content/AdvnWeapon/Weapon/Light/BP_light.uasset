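; BP_light is a weapon actor whose sphere displays the player's current weapon charge through its material.
; On BeginPlay it applies a dynamic instance of M_LightCharge to the sphere and starts a fast looping timer.
; Each tick of the timer reads ChargeAmount from player 0's BP_Weapon_Component, maps it through EmmisiveCurve and writes the result to the material's Amount parameter.
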(event EventBeginPlay
  (bind _returnvalue (Rendering|Material|CreateDynamicMaterialInstance "/Game/AdvnWeapon/Weapon/Light/M_LightCharge.M_LightCharge" "None" "None" :!class /Script/Engine.KismetMaterialLibrary))
  (bind _output_get (Variables|Default|SetMaterialRef _returnvalue))
  (Rendering|Material|SetMaterial (Variables|Default|GetSphere) 0 _output_get)
  (Utilities|Time|SetTimerbyFunctionName 0 "GetCurrentEmmisiveAmount" 0.01 true))

(fn ConstructionScript)

(fn GetCurrentEmmisiveAmount
  (bind _emmisivecurve (Variables|Default|GetEmmisiveCurve))
  (Utilities|IsValid _emmisivecurve
    (:Is%20Valid
      (bind _output_get (Variables|Default|SetEmissive%20Vaule (Math|Curves|GetFloatValue _emmisivecurve (Variables|/Game/AdvnWeapon/Weapon/BP_Weapon_Component.BP_Weapon_Component_C|GetChargeAmount (Actor|GetComponentbyClass (Game|GetPlayerCharacter 0) "/Game/AdvnWeapon/Weapon/BP_Weapon_Component.BP_Weapon_Component_C")))))
      (CallFunction|CurrentChargeStrenght _output_get))))

(fn CurrentChargeStrenght
  (params (CurrentCharge :type Float%20%28double-precision%29))
  (Rendering|Material|SetScalarParameterValue (Variables|Default|GetMaterialRef) "Amount" CurrentCharge :!class /Script/Engine.MaterialInstanceDynamic))