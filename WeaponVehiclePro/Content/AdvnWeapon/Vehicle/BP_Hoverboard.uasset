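; Rideable physics hoverboard that the player steers through Enhanced Input until exiting on a debug key.
; Hold time samples a speed curve for forward force on the Cube, a timer winds it down on release, and left/right apply yaw torque.
; COMHoverCharge gates forward thrust and feeds the vehicle HUD through an interface.
; Exiting repossesses the character and converts board speed into a player boost through two curves.
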(event OnComponentBeginOverlap(Sphere)
  (params (OverlappedComponent :type Primitive%20Component%20Object%20Reference) (OtherActor :type Actor%20Object%20Reference) (OtherComp :type Primitive%20Component%20Object%20Reference) (OtherBodyIndex :type Integer) (bFromSweep :type Boolean) (SweepResult :type Hit%20Result%20Structure%20%28by%20ref%29))
  (bind _asbp_player_character (Utilities|Casting|CastToBP_PlayerCharacter OtherActor))
  (bind _output_get (Variables|Default|SetCharRef _asbp_player_character))
  (EventDispatchers|BindEventtoInteract _output_get (delegate Custom|Take%20COntrol)))

(event OnComponentEndOverlap(Sphere)
  (params (OverlappedComponent :type Primitive%20Component%20Object%20Reference) (OtherActor :type Actor%20Object%20Reference) (OtherComp :type Primitive%20Component%20Object%20Reference) (OtherBodyIndex :type Integer))
  (bind _asbp_player_character (Utilities|Casting|CastToBP_PlayerCharacter OtherActor))
  (EventDispatchers|UnbindallEventsfromInteract _asbp_player_character))

(event Custom|Take%20COntrol)

(event Custom|Hover%20Update)

(event Custom|Forward%20Update
  (Variables|Default|SetTimeHeld (+ (Variables|Default|GetTimeHeld) 1.0)))

(event Custom|Vichle%20Slow%20Down
  (if (<= (Variables|Default|GetHeld%20Seconds) 0.0)
    (Utilities|Time|ClearandInvalidateTimerbyHandle (stale Input|EnhancedActionEvents|EnhancedInputActionIA_Forward _returnvalue))
    (Variables|Default|SetHeld%20Seconds 0.0)
    (else
      (bind _output_get (Variables|Default|SetHeld%20Seconds (- (Variables|Default|GetHeld%20Seconds) 0.1)))
      (bind _currentviechlespeed (CallFunction|GetVeichleSpeedCureve _output_get))
      (Variables|Default|SetForwardForce _currentviechlespeed))))

(event Custom|Init
  (bind _asbp_player_controller (Utilities|Casting|CastToBP_PlayerController (Game|GetPlayerController 0)))
  (Utilities|IsValid (PlayerController|LocalPlayerSubsystems|GetEnhancedInputLocalPlayerSubsystem _asbp_player_controller)
    (:Is%20Valid
      (Input|AddMappingContext (PlayerController|LocalPlayerSubsystems|GetEnhancedInputLocalPlayerSubsystem _asbp_player_controller) "/Game/AdvnWeapon/Input/IMC_Vichle.IMC_Vichle" 0 "(bIgnoreAllPressedKeysUntilRelease=True,bForceImmediately=False)")
      (Default|InitVehicle (Variables|/Game/AdvnWeapon/Character/BP_PlayerCharacter.BP_PlayerCharacter_C|GetCOM_MovemntAccelleration (Variables|Default|GetCharRefs)))
      (Variables|Default|SetCurrentState "NewEnumerator1")
      (Rendering|SetVisibility (Variables|Default|GetCube) true false)
      (Physics|AddForce (Variables|Default|GetCube) (* (Transformation|GetActorForwardVector) 7e+06 1.2) "None" false)
      (Utilities|FlowControl|Delay 1.0)
      (bind _returnvalue (UserInterface|CreateWidget "/Game/AdvnWeapon/UI/VehicleUI/WBP_MasterVehcle.WBP_MasterVehcle_C"))
      (UserInterface|Viewport|AddtoViewport _returnvalue 0)
      (Utilities|Time|SetTimerbyEvent (delegate Custom|CustomEvent) 0.01 true)
      (Default|ChargeCheck (Variables|Default|GetCOM_HoverCharge) (Variables|Default|GetCurrentState)))
    (:Is%20Not%20Valid
      (Development|PrintString "Hello"))))

(event Custom|CustomEvent
  (bind _foundwidgets (Class|WidgetBlueprintLibrary|GetAllWidgetswithInterface "/Game/AdvnWeapon/Vehicle/BPI_GetCurrentCharge.BPI_GetCurrentCharge_C" false))
  (for _array_element _foundwidgets
    (Utilities|IsValid _array_element
      (:Is%20Valid
        (Class|BPIGetCurrentCharge|VehicleCharge(Message) _array_element (Variables|/Game/AdvnWeapon/Vehicle/Charge/COM_HoverCharge.COM_HoverCharge_C|GetCurrent%20Charge (Variables|Default|GetCOM_HoverCharge)))))))

(event Input|EnhancedActionEvents|EnhancedInputActionIA_Back
  (params (ActionValue :type Boolean) (ElapsedSeconds :type Float%20%28double-precision%29) (TriggeredSeconds :type Float%20%28double-precision%29) (InputAction :type Input%20Action%20Object%20Reference :default "/Game/AdvnWeapon/Input/Veichle/IA_Back.IA_Back"))
  (:Ongoing
    (if (Utilities|Enum|Equal(Enum) (Variables|Default|GetCurrentState) "NewEnumerator1")
      (Physics|AddForce (Variables|Default|GetCube) (* (Transformation|GetActorForwardVector) (Variables|Default|GetForwardForce) -1.2) "None" false))))

(event Input|EnhancedActionEvents|EnhancedInputActionIA_Forward
  (params (ActionValue :type Boolean) (ElapsedSeconds :type Float%20%28double-precision%29) (TriggeredSeconds :type Float%20%28double-precision%29) (InputAction :type Input%20Action%20Object%20Reference :default "/Game/AdvnWeapon/Input/Veichle/IA_Forward.IA_Forward"))
  (:Started
    (bind _is_charge_0 (CallFunction|CheckCharge))
    (if (not _is_charge_0)
      (Default|InitLoseCharge (Variables|Default|GetCOM_HoverCharge))))
  (:Ongoing
    (bind _is_charge_0_2 (CallFunction|CheckCharge))
    (if (not _is_charge_0_2)
      (if (Utilities|Enum|Equal(Enum) (Variables|Default|GetCurrentState) "NewEnumerator1")
        (if (Utilities|Time|IsTimerActivebyHandle (stale _returnvalue))
          (Utilities|Time|ClearandInvalidateTimerbyHandle (stale _returnvalue)))
        (bind _output_get (Variables|Default|SetHeld%20Seconds ElapsedSeconds))
        (if (>= _output_get 6.0)
          (Variables|Default|SetHeld%20Seconds 6.0)
          (else
            (bind _currentviechlespeed (CallFunction|GetVeichleSpeedCureve _output_get))))
        (Variables|Default|SetForwardForce _currentviechlespeed)
        (Physics|AddForce (Variables|Default|GetCube) (* (Transformation|GetActorForwardVector) (Variables|Default|GetForwardForce)) "None" false))))
  (:Completed
    (Default|InitStopChargeLoss (Variables|Default|GetCOM_HoverCharge))
    (bind _returnvalue (Utilities|Time|SetTimerbyEvent (delegate Custom|Vichle%20Slow%20Down) 0.1 true))))

(event Input|EnhancedActionEvents|EnhancedInputActionIA_Right
  (params (ActionValue :type Boolean) (ElapsedSeconds :type Float%20%28double-precision%29) (TriggeredSeconds :type Float%20%28double-precision%29) (InputAction :type Input%20Action%20Object%20Reference :default "/Game/AdvnWeapon/Input/Veichle/IA_Right.IA_Right"))
  (:Triggered
    (Variables|Default|SetturnTorque 2e+08)
    (Class|PrimitiveComponent|AddTorqueinDegrees (Variables|Default|GetCube) (* (Transformation|GetActorUpVector) (Variables|Default|GetturnTorque)) "None" false :!label _label))
  (:Completed
    (Variables|Default|SetturnTorque 0.0)
    (goto _label)))

(event Input|EnhancedActionEvents|EnhancedInputActionIA_Left
  (params (ActionValue :type Boolean) (ElapsedSeconds :type Float%20%28double-precision%29) (TriggeredSeconds :type Float%20%28double-precision%29) (InputAction :type Input%20Action%20Object%20Reference :default "/Game/AdvnWeapon/Input/Veichle/IA_Left.IA_Left"))
  (:Triggered
    (Variables|Default|SetturnTorque -2e+08)
    (Class|PrimitiveComponent|AddTorqueinDegrees (Variables|Default|GetCube) (* (Transformation|GetActorUpVector) (Variables|Default|GetturnTorque)) "None" false :!label _label))
  (:Completed
    (Variables|Default|SetturnTorque 0.0)
    (goto _label)))

(event EventBeginPlay
  (bind _asbp_player_character (Utilities|Casting|CastToBP_PlayerCharacter (Game|GetPlayerCharacter 0)))
  (Variables|Default|SetCharRefs _asbp_player_character)
  (Variables|Default|SetCurrentState "NewEnumerator1"))

(event EventPossessed
  (params (NewController :type Controller%20Object%20Reference)))

(event EventUnpossessed
  (params (OldController :type Controller%20Object%20Reference)))

(event Input|KeyboardEvents|DebugKeyW
  (params (Key :type Key%20Structure :default "None") (ActionValue :type Input%20Action%20Value%20Structure)))

(event Input|KeyboardEvents|DebugKeyS
  (params (Key :type Key%20Structure :default "None") (ActionValue :type Input%20Action%20Value%20Structure)))

(event Input|KeyboardEvents|DebugKeyA
  (params (Key :type Key%20Structure :default "None") (ActionValue :type Input%20Action%20Value%20Structure)))

(event Input|KeyboardEvents|DebugKeyD
  (params (Key :type Key%20Structure :default "None") (ActionValue :type Input%20Action%20Value%20Structure)))

(event Input|KeyboardEvents|DebugKeyW
  (params (Key :type Key%20Structure :default "None") (ActionValue :type Input%20Action%20Value%20Structure)))

(event Input|KeyboardEvents|DebugKeyS
  (params (Key :type Key%20Structure :default "None") (ActionValue :type Input%20Action%20Value%20Structure)))

(event Input|KeyboardEvents|DebugKeyD
  (params (Key :type Key%20Structure :default "None") (ActionValue :type Input%20Action%20Value%20Structure)))

(event Input|KeyboardEvents|DebugKeyA
  (params (Key :type Key%20Structure :default "None") (ActionValue :type Input%20Action%20Value%20Structure)))

(event Input|KeyboardEvents|DebugKeyE
  (params (Key :type Key%20Structure :default "None") (ActionValue :type Input%20Action%20Value%20Structure))
  (bind _charrefs (Variables|Default|GetCharRefs))
  (bind _charrefs_2 (Variables|Default|GetCharRefs))
  (:Pressed
    (Utilities|IsValid _charrefs_2
      (:Is%20Valid
        (Collision|SetActorEnableCollision _charrefs true)
        (Rendering|SetActorHiddenInGame _charrefs false)
        (Transformation|Teleport (Variables|Default|GetCharRefs) (Transformation|GetWorldLocation (Variables|Default|GetPlayerPoint)) (Math|Conversions|RotationFromXVector (Math|Vector|GetForwardVector (Variables|Default|GetCube))))
        (Default|ChargeCheck (Variables|Default|GetCOM_HoverCharge) "NewEnumerator0")
        (Pawn|Possess (Game|GetPlayerController 0) _charrefs_2)
        (Variables|Default|SetCurrentState "NewEnumerator0")
        (Rendering|SetVisibility (Variables|Default|GetCube) false false)
        (Viewport|RemoveAllWidgets)
        (Default|SetupUI _charrefs_2)
        (bind _boostamount (CallFunction|FindVehiclePlayerBoost))
        (Default|OnEventVehileSpeedBost (Variables|Default|GetCharRefs) _boostamount)))))

(fn ConstructionScript)

(fn GetVeichleSpeedCureve
  (params (IncomingSeconds :type Float%20%28double-precision%29))
  (return (Math|Curves|GetFloatValue (Variables|Default|GetVehicleSpeedCurve) IncomingSeconds)))

(fn CheckCharge
  (return (<= (Variables|/Game/AdvnWeapon/Vehicle/Charge/COM_HoverCharge.COM_HoverCharge_C|GetCurrent%20Charge (Variables|Default|GetCOM_HoverCharge)) 0.0)))

(fn FindVehcielSpeedPercent
  (return (Math|Curves|GetFloatValue (Variables|Default|GetCurve_FindvehicleSpeedPercent) (Variables|Default|GetForwardForce))))

(fn FindVehiclePlayerBoost
  (bind _percent (CallFunction|FindVehcielSpeedPercent))
  (return (Math|Curves|GetFloatValue (Variables|Default|GetCurve_VehicleToPlayer) _percent)))