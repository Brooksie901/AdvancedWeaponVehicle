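; BP_SceneCheck is a scene component on BP_Hoverboard that adjusts hover height for the surface below.
; Each tick it runs a debug-drawn Visibility line trace along its local down axis.
; On a hit, it sets every BP_HoverComponent on the owner to a higher hover distance for components tagged "water", and a lower one otherwise.
; With no hit, the hover distances stay unchanged.
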(event EventBeginPlay
  (bind _asbp_hoverboard (Utilities|Casting|CastToBP_Hoverboard (Components|GetOwner)))
  (Variables|Default|SetParent _asbp_hoverboard))

(event EventTick
  (params (DeltaSeconds :type Float%20%28single-precision%29))
  (bind _returnvalue (Transformation|GetWorldLocation))
  (bind _returnvalue_2 (Components|GetOwner))
  (bind _returnvalue_3 (Actor|GetComponentsByClass _returnvalue_2 "/Game/AdvnWeapon/Vehicle/BP_HoverComponent.BP_HoverComponent_C"))
  (Utilities|IsValid (Variables|Default|GetParent)
    (:Is%20Valid
      (bind (_outhit _returnvalue_4) (Collision|LineTraceByChannel _returnvalue (- _returnvalue (* (Math|Vector|GetUpVector) (Variables|Default|GetHoverDistance))) "TraceTypeQuery1" false 0 "ForOneFrame"))
      (if _returnvalue_4
        (if (Components|ComponentHasTag (.HitComponent (Collision|BreakHitResult _outhit)) "water")
          (for _array_element _returnvalue_3
            (Variables|/Game/AdvnWeapon/Vehicle/BP_HoverComponent.BP_HoverComponent_C|SetHoverDistance _array_element 3e+02))
          (else
            (for _array_element_2 _returnvalue_3
              (Variables|/Game/AdvnWeapon/Vehicle/BP_HoverComponent.BP_HoverComponent_C|SetHoverDistance _array_element_2 2e+02))))))))