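; Hover point component for BP_Hoverboard that pushes the board's root primitive away from the surface beneath it.
; Each tick it traces down along its up vector for the hover distance, with debug drawing on.
; On a hit it applies force at its location along the surface normal, fading linearly with distance, and sets fixed linear and angular damping.
; An alternative spring-damper version remains in the graph but never runs.
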(event EventBeginPlay
  (bind _asbp_hoverboard (Utilities|Casting|CastToBP_Hoverboard (Components|GetOwner)))
  (Variables|Default|SetParent _asbp_hoverboard))

(event EventTick
  (params (DeltaSeconds :type Float%20%28single-precision%29))
  (bind _returnvalue (Transformation|GetWorldLocation))
  (bind _parent (Variables|Default|GetParent))
  (bind _rootcomponent (Variables|/Script/Engine.Actor|GetRootComponent _parent))
  (bind _asprimitive_component (Utilities|Casting|CastToPrimitiveComponent _rootcomponent))
  (Utilities|IsValid (Variables|Default|GetParent)
    (:Is%20Valid
      (bind (_outhit _returnvalue_2) (Collision|LineTraceByChannel _returnvalue (- _returnvalue (* (Math|Vector|GetUpVector) (Variables|Default|GetHoverDistance))) "TraceTypeQuery1" false 0 "ForOneFrame"))
      (if _returnvalue_2
        (Utilities|IsValid _asprimitive_component
          (:Is%20Valid
            (Class|PrimitiveComponent|AddForceatLocation _asprimitive_component (* (.ImpactNormal (Collision|BreakHitResult _outhit)) (Math|Float|Lerp (Variables|Default|GetForce) 0.0 (/ (Math|Vector|VectorLength (- (.Location (Collision|BreakHitResult _outhit)) (Transformation|GetWorldLocation))) (Variables|Default|GetHoverDistance)))) (Transformation|GetWorldLocation) "None")
            (Class|PrimitiveComponent|SetLinearDamping _asprimitive_component 2.0)
            (Class|PrimitiveComponent|SetAngularDamping _asprimitive_component 3.0)))))))