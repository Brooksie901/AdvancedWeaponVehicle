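; BP_SlowArea is a trigger volume that applies a slow effect to actors while they are inside it.
; Box overlap begin and end events check that the actor implements BPI_Slow and has a valid COM_Slow component.
; They then call SlowMessage on entry and SlowEndMessage on exit on that component, which handles the slowing itself.
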(event OnComponentBeginOverlap(Box)
  (params (OverlappedComponent :type Primitive%20Component%20Object%20Reference) (OtherActor :type Actor%20Object%20Reference) (OtherComp :type Primitive%20Component%20Object%20Reference) (OtherBodyIndex :type Integer) (bFromSweep :type Boolean) (SweepResult :type Hit%20Result%20Structure%20%28by%20ref%29))
  (bind _returnvalue (Actor|GetComponentbyClass OtherActor "/Game/Slow/COM_Slow.COM_Slow_C"))
  (if (Utilities|DoesObjectImplementInterface OtherActor "/Game/Slow/BPI_Slow.BPI_Slow_C")
    (Utilities|IsValid _returnvalue
      (:Is%20Valid
        (Class|BPISlow|Slow(Message) _returnvalue)))))

(event OnComponentEndOverlap(Box)
  (params (OverlappedComponent :type Primitive%20Component%20Object%20Reference) (OtherActor :type Actor%20Object%20Reference) (OtherComp :type Primitive%20Component%20Object%20Reference) (OtherBodyIndex :type Integer))
  (bind _returnvalue (Actor|GetComponentbyClass OtherActor "/Game/Slow/COM_Slow.COM_Slow_C"))
  (if (Utilities|DoesObjectImplementInterface OtherActor "/Game/Slow/BPI_Slow.BPI_Slow_C")
    (Utilities|IsValid _returnvalue
      (:Is%20Valid
        (Class|BPISlow|SlowEnd(Message) _returnvalue)))))

(event EventBeginPlay)

(fn ConstructionScript)